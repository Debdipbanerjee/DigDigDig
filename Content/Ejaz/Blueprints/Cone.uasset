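; Cone is an actor Blueprint that spins around its local X (roll) axis while switched on.
; StartRotating and StopRotating set a Rotating flag, and the construction script calls StopRotating so it begins idle.
; While the flag is set, Tick adds a local roll each frame at MaxRotSpeed scaled by delta time.
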(event `self.ReceiveTick`
  (params (DeltaSeconds :type "Float (single-precision)"))
  (if (`self.rotating`)
    (`self.K2_AddActorLocalRotation` (* (`KismetMathLibrary.MakeRotator` (`self.maxRotSpeed`)) DeltaSeconds))))

(fn `StartRotating`
  (set `self.rotating` true))

(fn `StopRotating`
  (set `self.rotating` false))

(fn `UserConstructionScript`
  (`self.StopRotating`))