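; Spawner actor that fills a three-dimensional grid with Bp_block actors when play begins.
; Nested loops over FieldHeight, FieldLength and FieldWidth map to Z, Y and X and call SpawnBlock for each cell.
; SpawnBlock scales the cell indices by BlockSpacing, then adds the root component's world location, so the field extends along positive world axes from the spawner without following its rotation.
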(event `self.ReceiveBeginPlay`
  (for _index (range (`self.fieldHeight`))
    (for _index_2 (range (`self.fieldLength`))
      (for _index_3 (range (`self.fieldWidth`))
        (`self.SpawnBlock` (`KismetMathLibrary.Conv_IntToDouble` _index_3) (`KismetMathLibrary.Conv_IntToDouble` _index_2) (`KismetMathLibrary.Conv_IntToDouble` _index))))))

(fn `Offset By Block Spacing`
  (params (x :type "Float (double-precision)") (y :type "Float (double-precision)") (z :type "Float (double-precision)"))
  (returns (offsetX :type "Float (double-precision)") (offsetY :type "Float (double-precision)") (offsetZ :type "Float (double-precision)"))
  (bind _blockspacing (`self.blockSpacing`))
  (return (* x _blockspacing) (* _blockspacing y) (* _blockspacing z)))

(fn `Offset By World Pos`
  (params (X :type "Float (double-precision)") (Y :type "Float (double-precision)") (Z :type "Float (double-precision)"))
  (returns (offsetX :type "Float (double-precision)") (offsetY :type "Float (double-precision)") (offsetZ :type "Float (double-precision)"))
  (bind (_returnvalue_x _returnvalue_y _returnvalue_z) (`KismetMathLibrary.BreakVector` (+ (`KismetMathLibrary.MakeVector` X Y Z) (`SceneComponent.K2_GetComponentLocation` (`self.DefaultSceneRoot`)))))
  (return _returnvalue_x _returnvalue_y _returnvalue_z))

(fn `SpawnBlock`
  (params (X :type "Float (double-precision)") (Y :type "Float (double-precision)") (Z :type "Float (double-precision)"))
  (bind (_offsetx _offsety _offsetz) (`self.Offset By Block Spacing` X Y Z))
  (bind (_offsetx_2 _offsety_2 _offsetz_2) (`self.Offset By World Pos` _offsetx _offsety _offsetz))
  (`|SpawnActorFromClass` "/Game/Blueprints/bp_block.bp_block_C" (`KismetMathLibrary.MakeTransform` (`KismetMathLibrary.MakeVector` _offsetx_2 _offsety_2 _offsetz_2)) "Undefined" "OverrideRootScale" null null))

(fn `UserConstructionScript`)