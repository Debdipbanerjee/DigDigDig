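; Drill tool Blueprint that starts and stops drilling as its use-tool input is pressed and released.
; On BeginPlay it casts the Cone child actor component's actor to the Cone class and caches it.
; Press and release events set a Drilling flag and tell that cone to start or stop rotating.
; No drilling effect beyond the flag and rotation calls is implemented in this graph.
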(event `self.ReceiveBeginPlay`
  (bind _ascone (cast `/Game/Ejaz/Blueprints/Cone` (`ChildActorComponent.ChildActor` (`self.Cone`))))
  (set `self.myCone` _ascone))

(event `self.ReceiveTick`
  (params (DeltaSeconds :type "Float (single-precision)")))

(event `self.UseToolPressed`
  (set `self.drilling` true)
  (`/Game/Ejaz/Blueprints/Cone.StartRotating` (`self.myCone`)))

(event `self.UseToolReleased`
  (set `self.drilling` false)
  (`/Game/Ejaz/Blueprints/Cone.StopRotating` (`self.myCone`)))

(fn `UserConstructionScript`
  (`parent.UserConstructionScript`))