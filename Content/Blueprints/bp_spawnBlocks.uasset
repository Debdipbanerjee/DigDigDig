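; Actor Blueprint that spawns a 3D grid of Bp_Cubes actors at runtime when play begins.
; BeginPlay runs three nested loops over GridSize for X and Y and GridHeight for Z, calling SpawnBlock for each cell.
; SpawnBlock scales each index by CubeSpacing and offsets it from the root component's world location, so the grid starts at the spawner's position.
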(event `self.ReceiveBeginPlay`
  (bind _gridsize (`self.GridSize`))
  (for _index (range (+ _gridsize 1))
    (for _index_2 (range (+ _gridsize 1))
      (for _index_3 (range (+ (`self.GridHeight`) 1))
        (`self.SpawnBlock` (`KismetMathLibrary.Conv_IntToDouble` _index) (`KismetMathLibrary.Conv_IntToDouble` _index_2) (`KismetMathLibrary.Conv_IntToDouble` _index_3))))))

(fn `Add To Own Location`
  (params (A :type "Float (double-precision)") (A2 :type "Float (double-precision)") (A3 :type "Float (double-precision)"))
  (returns (ReturnValue :type "Float (double-precision)") (ReturnValue2 :type "Float (double-precision)") (ReturnValue3 :type "Float (double-precision)"))
  (bind (_returnvalue_x _returnvalue_y _returnvalue_z) (`KismetMathLibrary.BreakVector` (`SceneComponent.K2_GetComponentLocation` (`self.DefaultSceneRoot`))))
  (return (+ A _returnvalue_x) (+ A2 _returnvalue_y) (+ A3 _returnvalue_z)))

(fn `multiply cube spacing`
  (params (value :type "Float (double-precision)"))
  (returns (output :type "Float (double-precision)"))
  (return (* value (`self.Cube Spacing`))))

(fn `SpawnBlock`
  (params (x :type "Float (double-precision)") (y :type "Float (double-precision)") (z :type "Float (double-precision)"))
  (bind (_returnvalue _returnvalue2 _returnvalue3) (`self.Add To Own Location` (`self.multiply cube spacing` x) (`self.multiply cube spacing` y) (`self.multiply cube spacing` z)))
  (`|SpawnActorFromClass` "/Game/Blueprints/bp_Cubes.bp_Cubes_C" (`KismetMathLibrary.MakeTransform` (`KismetMathLibrary.MakeVector` _returnvalue _returnvalue2 _returnvalue3)) "Undefined" "OverrideRootScale" null null))

(fn `UserConstructionScript`)