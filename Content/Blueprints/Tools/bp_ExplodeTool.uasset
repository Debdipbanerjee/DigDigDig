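; Tool actor that blasts away nearby Cube_Blueprint actors when the Explode input is pressed.
; The input calls UseToolPressed, which gathers every Cube_Blueprint in the level with GetAllActorsOfClass.
; Each cube whose root component lies within ExplodeRadium of the tool's location is destroyed, with no physics or effects.
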(event `InputAction|Explode`
  (params (Key :type "Key Structure"))
  (:`Pressed`
    (`self.UseToolPressed`)))

(fn `UserConstructionScript`
  (`parent.UserConstructionScript`))

(fn `UseToolPressed`
  ;[1 1 1] Explode
  (bind _outactors (`GameplayStatics.GetAllActorsOfClass` "/Game/Blueprints/Cube_Blueprint.Cube_Blueprint_C"))
  (for _array_element _outactors
    (if (< (`KismetMathLibrary.VSize` (- (`SceneComponent.K2_GetComponentLocation` (`Actor.RootComponent` _array_element)) (`self.K2_GetActorLocation`))) (`self.explodeRadium`))
      (`/Game/Blueprints/Cube_Blueprint.Destroy` _array_element))))